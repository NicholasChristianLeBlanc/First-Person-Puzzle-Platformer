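; Physics pickup block that can grow in size and mass while its speed stays capped.
; Each Grow event adds GrowthRate to the actor's scale and the mesh's mass scale, using MaxScale as the limit for both.
; Every tick, ConstrainVelocity rescales the mesh's linear velocity to MaxVelocity when it goes faster, preserving its direction.
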(event `self.ReceiveBeginPlay`)

(event `self.ReceiveTick`
  (params (DeltaSeconds :type "Float (single-precision)"))
  (`self.Constrain Velocity`))

(event `Grow`
  (bind _staticmeshcomponent (`self.StaticMeshComponent`))
  (bind _max_scale (`self.Max Scale`))
  (bind _growth_rate (`self.Growth Rate`))
  (bind _returnvalue (+ (`self.GetActorScale3D`) (`KismetMathLibrary.Conv_DoubleToVector` _growth_rate)))
  (bind _returnvalue_2 (+ (`PrimitiveComponent.GetMassScale` _staticmeshcomponent "None") _growth_rate))
  (if (or (>= (.x _returnvalue) _max_scale) (>= (.y _returnvalue) _max_scale) (>= (.z _returnvalue) _max_scale))
    (`self.SetActorScale3D` (`KismetMathLibrary.Conv_DoubleToVector` _max_scale))
    (else
      (`self.SetActorScale3D` _returnvalue)))
  (if (>= _returnvalue_2 _max_scale)
    (`PrimitiveComponent.SetMassScale` _staticmeshcomponent "None" (`self.Max Scale`))
    (else
      (`PrimitiveComponent.SetMassScale` _staticmeshcomponent "None" _returnvalue_2))))

(fn `Constrain Velocity`
  (bind _max_velocity (`self.Max Velocity`))
  (bind _returnvalue (`PrimitiveComponent.GetPhysicsLinearVelocity` (`self.StaticMeshComponent`) "None"))
  (bind _returnvalue_2 (`KismetMathLibrary.VSize` _returnvalue))
  (if (< _max_velocity _returnvalue_2)
    (`PrimitiveComponent.SetPhysicsLinearVelocity` (`self.StaticMeshComponent`) (* _returnvalue (/ _max_velocity _returnvalue_2)) false "None")))

(fn `UserConstructionScript`)