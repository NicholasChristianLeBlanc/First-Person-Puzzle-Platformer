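; A switch actor that becomes active when hit, except by grow or shrink projectiles.
; On a hit it destroys standard first-person projectiles and sets a WasHit flag, which GetActive exposes to other objects.
; A nonzero ActiveTime resets the flag after that absolute delay; zero leaves the switch on.
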(event `self.ReceiveBeginPlay`)

(event `self.ReceiveHit`
  (params (MyComp :type "PrimitiveComponent Object Reference") (Other :type "Actor Object Reference") (OtherComp :type "PrimitiveComponent Object Reference") (bSelfMoved :type Boolean) (HitLocation :type "Vector Structure") (HitNormal :type "Vector Structure") (NormalImpulse :type "Vector Structure") (Hit :type "HitResult Structure (by ref)"))
  (bind _returnvalue (`GameplayStatics.GetObjectClass` Other))
  (if (and (!= _returnvalue "/Game/MainGame/Blueprints/ProjectileGrowObjects.ProjectileGrowObjects_C") (!= _returnvalue "/Game/MainGame/Blueprints/ProjectileShrinkObjects.ProjectileShrinkObjects_C"))
    (if (== (`GameplayStatics.GetObjectClass` Other) "/Game/MainGame/Blueprints/FirstPersonProjectile.FirstPersonProjectile_C")
      (`self.K2_DestroyActor` Other))
    (`self.Was Triggered`)))

(event `Was Triggered`
  (bind _returnvalue (`KismetMathLibrary.Abs` (`self.Active Time`)))
  (set `self.Was Hit` true)
  (if (> _returnvalue 0.0)
    (`KismetSystemLibrary.Delay` _returnvalue)
    (set `self.Was Hit` false)))

(fn `Get Active`
  (returns (`Is Active` :type Boolean))
  (return (`self.Was Hit`)))

(fn `UserConstructionScript`)