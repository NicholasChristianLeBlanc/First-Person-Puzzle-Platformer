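; Door actor that opens by hiding its static mesh and disabling its collision, and closes by restoring both.
; BeginPlay applies the initial Active state, with active meaning open.
; SetActive updates Active and re-applies that state, but a DoorFailure flag keeps the mesh unchanged when activating, while deactivating always closes the door.
; BeginPlay ignores DoorFailure, so a door starting active opens regardless.
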(event `self.ReceiveBeginPlay`
  (bind _staticmesh (`self.StaticMesh`))
  (if (`self.Active`)
    (`PrimitiveComponent.SetCollisionEnabled` _staticmesh "NoCollision")
    (`SceneComponent.SetHiddenInGame` _staticmesh true false)
    (else
      (`PrimitiveComponent.SetCollisionEnabled` _staticmesh "QueryAndPhysics")
      (`SceneComponent.SetHiddenInGame` _staticmesh false false))))

(fn `Set Active`
  (params (`New Active` :type Boolean))
  (bind _staticmesh (`self.StaticMesh`))
  (bind _output_get (set `self.Active` `New Active`))
  (if _output_get
    (if (not (`self.Door Failure`))
      (`PrimitiveComponent.SetCollisionEnabled` _staticmesh "NoCollision")
      (`SceneComponent.SetHiddenInGame` _staticmesh true false))
    (else
      (`PrimitiveComponent.SetCollisionEnabled` _staticmesh "QueryAndPhysics")
      (`SceneComponent.SetHiddenInGame` _staticmesh false false))))

(fn `UserConstructionScript`)