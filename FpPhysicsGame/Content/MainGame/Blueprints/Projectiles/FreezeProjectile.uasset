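; Freeze projectile that turns death water into temporary standing platforms on contact.
; On overlapping DeathWater that is not animating, it spawns a FreezePlatform just above the water box at the impact XY and passes it the melt time.
; Setters configure the melt time and whether the platform attaches to the water actor.
; The projectile destroys itself after any death water overlap, while other actors are ignored.
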(event `self.ReceiveActorBeginOverlap`
  (params (OtherActor :type "Actor Object Reference"))
  (bind (_returnvalue_x _returnvalue_y) (`KismetMathLibrary.BreakVector` (`self.K2_GetActorLocation`)))
  (bind _asdeath_water (cast `/Game/MainGame/Blueprints/InteractiveObjects/DeathWater` OtherActor))
  (if (not (`/Game/MainGame/Blueprints/InteractiveObjects/DeathWater.Animating` _asdeath_water))
    (bind (_returnvalue_x_2 _returnvalue_y_2 _returnvalue_z) (`KismetMathLibrary.BreakVector` (`SceneComponent.GetSocketLocation` (`/Game/MainGame/Blueprints/InteractiveObjects/DeathWater.Box` _asdeath_water) "None")))
    (bind _returnvalue (`|SpawnActorFromClass` "/Game/MainGame/Blueprints/InteractiveObjects/FreezePlatform.FreezePlatform_C" (`KismetMathLibrary.Conv_VectorToTransform` (`KismetMathLibrary.MakeVector` _returnvalue_x _returnvalue_y (+ _returnvalue_z 5.0))) "Undefined" "OverrideRootScale" null null))
    (`/Game/MainGame/Blueprints/InteractiveObjects/FreezePlatform.Set Melt Time` _returnvalue (`self.PlatformMeltTime`))
    (if (not (not (`self.PlatformParentToWater`)))
      (`self.K2_AttachToActor` _returnvalue OtherActor "None" "KeepWorld" "KeepWorld" "KeepWorld" false)))
  (`self.K2_DestroyActor`))

(fn `Set Melt Time`
  (params (`New Melt Time` :type "Float (double-precision)"))
  (set `self.PlatformMeltTime` `New Melt Time`))

(fn `Set Platform Parent Bool`
  (params (NewBool :type Boolean))
  (set `self.PlatformParentToWater` NewBool))

(fn `UserConstructionScript`)