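; Projectile that shrinks Pickup_Block actors it hits, then destroys itself; hits on other classes are ignored.
; Each hit adds ShrinkRate to the block's 3D scale and to the hit component's mass scale, clamping both at MinScale.
; The Vector Comparison helper is meant to flag when any scale axis reaches the minimum, triggering a uniform clamp on the actor scale.
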(event `self.ReceiveHit`
  (params (MyComp :type "PrimitiveComponent Object Reference") (Other :type "Actor Object Reference") (OtherComp :type "PrimitiveComponent Object Reference") (bSelfMoved :type Boolean) (HitLocation :type "Vector Structure") (HitNormal :type "Vector Structure") (NormalImpulse :type "Vector Structure") (Hit :type "HitResult Structure (by ref)"))
  (bind _min_scale (`self.Min Scale`))
  (bind _shrink_rate (`self.Shrink Rate`))
  (bind _returnvalue (+ (`PrimitiveComponent.GetMassScale` OtherComp "None") _shrink_rate))
  (bind _returnvalue_2 (+ (`self.GetActorScale3D` Other) (`KismetMathLibrary.Conv_DoubleToVector` _shrink_rate)))
  (if (== (`GameplayStatics.GetObjectClass` Other) "/Game/MainGame/Blueprints/InteractiveObjects/Pickup_Block.Pickup_Block_C")
    (if (or (<= (.x _returnvalue_2) _min_scale) (<= (.y _returnvalue_2) _min_scale) (<= (.z _returnvalue_2) _min_scale))
      (`self.SetActorScale3D` Other (`KismetMathLibrary.Conv_DoubleToVector` _min_scale))
      (else
        (`self.SetActorScale3D` Other _returnvalue_2)))
    (if (<= _returnvalue _min_scale)
      (`PrimitiveComponent.SetMassScale` OtherComp "None" (`self.Min Scale`))
      (else
        (`PrimitiveComponent.SetMassScale` OtherComp "None" _returnvalue)))
    (`self.K2_DestroyActor`)))

(fn `UserConstructionScript`)