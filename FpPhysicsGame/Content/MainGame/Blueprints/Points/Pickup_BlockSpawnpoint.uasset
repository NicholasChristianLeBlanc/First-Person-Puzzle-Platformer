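; Spawn point that creates and respawns a Pickup_Block at its Box component's location and rotation.
; On Activate it respawns its existing block, or spawns one if none is valid, and registers itself as that block's RespawnPoint.
; An Active flag with a one-second delay ignores repeat activations during the cooldown.
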(event `Activate`
  (bind _box (`self.Box`))
  (bind _spawned_block (`self.Spawned Block`))
  (if (not (`self.Active`))
    (set `self.Active` true)
    (`/Engine/EditorBlueprintResources/StandardMacros.IsValid` _spawned_block
      (:`Is Valid`
        (`/Game/MainGame/Blueprints/InteractiveObjects/Pickup_Block.Respawn` _spawned_block))
      (:`Is Not Valid`
        (bind _returnvalue (`|SpawnActorFromClass` "/Game/MainGame/Blueprints/InteractiveObjects/Pickup_Block.Pickup_Block_C" (`KismetMathLibrary.MakeTransform` (`SceneComponent.K2_GetComponentLocation` _box) (`SceneComponent.K2_GetComponentRotation` _box)) "Undefined" "OverrideRootScale" null null))
        (set `/Game/MainGame/Blueprints/InteractiveObjects/Pickup_Block.RespawnPoint` self _returnvalue)
        (set `self.Spawned Block` _returnvalue)))
    (`KismetSystemLibrary.Delay` 1.0)
    (set `self.Active` false)))

(fn `UserConstructionScript`)