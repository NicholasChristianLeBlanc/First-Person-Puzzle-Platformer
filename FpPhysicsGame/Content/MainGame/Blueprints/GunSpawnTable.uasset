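; Gun spawn table actor that displays a gun mesh and records when the player reaches it.
; Tick polls the sphere collider for player pawn overlap, then sets a one-way PlayerCollide flag and hides the gun.
; ReturnCollisionEnter exposes that flag.
; IsObservable, unused within this graph, reports whether a visibility trace from a skeletal mesh to the player controller's location is unblocked.
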(event `self.ReceiveTick`
  (params (DeltaSeconds :type "Float (single-precision)"))
  (if (`self.Player Collide`)
    _
    (elif (`PrimitiveComponent.IsOverlappingActor` (`self.Sphere Collider`) (`GameplayStatics.GetPlayerPawn` 0))
      (set `self.Player Collide` true)
      (`SceneComponent.SetHiddenInGame` (`self.Gun Mesh`) true false))))

(fn `Is Observable`
  (params (`Skeletal Mesh` :type "SkeletalMeshComponent Object Reference"))
  (returns (`Is Observable` :type Boolean))
  (bind (_outhit _returnvalue) (`KismetSystemLibrary.LineTraceSingle` :`Start` (`SceneComponent.K2_GetComponentLocation` `Skeletal Mesh`) :`End` (`self.K2_GetActorLocation` (`GameplayStatics.GetPlayerController` 0)) :`TraceChannel` "TraceTypeQuery1" :`bIgnoreSelf` false))
  (return (not _returnvalue)))

(fn `Return collision enter`
  (returns (`Player Entered Zone` :type Boolean))
  (return (`self.Player Collide`)))

(fn `UserConstructionScript`)