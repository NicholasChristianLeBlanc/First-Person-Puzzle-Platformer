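; Physics block that the player can pick up, launch and, if scaleable, grow or shrink, with mass following scale.
; Tick caps velocity and blocks pickup when oversized; launched blocks instead get slight horizontal damping until hitting a StaticMeshActor.
; Grow first checks box overlaps for room, discounting other blocks, and a sphere flags player contact.
; Respawn resets scale, mass and motion at its spawn point, forcing a held block's drop, or destroys it without one.
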(event `self.ReceiveBeginPlay`
  (bind _staticmeshcomponent (`self.StaticMeshComponent`))
  (bind _staticmeshcomponent_2 (`self.StaticMeshComponent`))
  (bind _min_mass (`self.Min Mass`))
  (bind _min_mass_2 (`self.Min Mass`))
  (bind _returnvalue_x (`KismetMathLibrary.BreakVector` (`SceneComponent.K2_GetComponentScale` _staticmeshcomponent)))
  ;[1 1 1] Begin Play
  (`PrimitiveComponent.SetPhysicsMaxAngularVelocityInDegrees` _staticmeshcomponent (`self.Max Rotation Velocity`) false "None")
  (`PrimitiveComponent.SetAngularDamping` _staticmeshcomponent 0.25)
  (if (and (`self.Scaleable`) (> _min_mass_2 0.0) (> (`self.Max Mass`) _min_mass_2))
    (if (and (>= _returnvalue_x (`self.Min Scale`)) (<= _returnvalue_x (`self.Max Scale`)))
      (set `self.Default Scale` _returnvalue_x))
    (if (and (> _min_mass 0.0) (> (`self.Max Mass`) _min_mass))
      (`PrimitiveComponent.SetMassOverrideInKg` _staticmeshcomponent_2 "None" (`KismetMathLibrary.Lerp` (`self.Min Mass`) (`self.Max Mass`) (`KismetMathLibrary.NormalizeToRange` _returnvalue_x (`self.Min Scale`) (`self.Max Mass`))) true)
      (else
        (`PrimitiveComponent.SetAllMassScale` _staticmeshcomponent_2 _returnvalue_x)))))

(event `self.ReceiveTick`
  (params (DeltaSeconds :type "Float (single-precision)"))
  (bind (_returnvalue_x _returnvalue_y _returnvalue_z) (`KismetMathLibrary.BreakVector` (`self.GetVelocity`)))
  (bind _pickup_max_scale (`self.Pickup Max Scale`))
  ;[1 1 1] Tick
  (if (not (`self.WasLaunched`))
    (`self.Constrain Velocity`)
    (if (not (`self.Force Non Pickup`))
      (if (or (> (.x (`self.GetActorScale3D`)) _pickup_max_scale) (> (.y (`self.GetActorScale3D`)) _pickup_max_scale) (> (.z (`self.GetActorScale3D`)) _pickup_max_scale))
        (set `self.Can Pickup` false)
        (else
          (set `self.Can Pickup` true)))
      (else
        (set `self.Can Pickup` false)))
    (else
      (`PrimitiveComponent.SetPhysicsLinearVelocity` (`self.StaticMeshComponent`) (`KismetMathLibrary.MakeVector` (* _returnvalue_x 0.9999) (* _returnvalue_y 0.9999) _returnvalue_z) false "None"))))

(event `Launch`
  (params (`Launch Velocity` :type "Vector Structure"))
  ;[1 1 1] Handles Launch Events
  (set `self.WasLaunched` true)
  (`PrimitiveComponent.AddImpulse` (`self.StaticMeshComponent`) `Launch Velocity` "None" true))

(event `self.Sphere.OnComponentBeginOverlap`
  (params (OverlappedComponent :type "PrimitiveComponent Object Reference") (OtherActor :type "Actor Object Reference") (OtherComp :type "PrimitiveComponent Object Reference") (OtherBodyIndex :type Integer) (bFromSweep :type Boolean) (SweepResult :type "HitResult Structure (by ref)"))
  ;[1 1 1] Check For Player Collision
  (if (== (`GameplayStatics.GetObjectClass` OtherActor) "/Game/MainGame/Blueprints/FirstPersonCharacter.FirstPersonCharacter_C")
    (set `self.Player Collision` true)
    (else
      (set `self.Player Collision` false :!label _label))))

(event `self.StaticMeshComponent.OnComponentHit`
  (params (HitComponent :type "PrimitiveComponent Object Reference") (OtherActor :type "Actor Object Reference") (OtherComp :type "PrimitiveComponent Object Reference") (NormalImpulse :type "Vector Structure") (Hit :type "HitResult Structure (by ref)"))
  ;[1 1 1] Handles Launch Events
  (cast `StaticMeshActor` OtherActor)
  (set `self.WasLaunched` false))

(event `self.Sphere.OnComponentEndOverlap`
  (params (OverlappedComponent :type "PrimitiveComponent Object Reference") (OtherActor :type "Actor Object Reference") (OtherComp :type "PrimitiveComponent Object Reference") (OtherBodyIndex :type Integer))
  ;[1 1 1] Check For Player Collision
  (goto _label))

(event `Respawn`
  (bind _staticmeshcomponent (`self.StaticMeshComponent`))
  (bind _respawnpoint (`self.RespawnPoint`))
  (bind _min_mass (`self.Min Mass`))
  (bind _default_scale (`self.Default Scale`))
  ;[1 1 1] Custom Events
  ;;[1 0 0] Respawn
  (`/Engine/EditorBlueprintResources/StandardMacros.IsValid` (`self.RespawnPoint`)
    (:`Is Valid`
      (if (and (`self.Scaleable`) (> _default_scale 0.0))
        (`self.SetActorScale3D` (`KismetMathLibrary.Conv_DoubleToVector` _default_scale)))
      (if (and (> _min_mass 0.0) (> (`self.Max Mass`) _min_mass))
        (`PrimitiveComponent.SetMassOverrideInKg` _staticmeshcomponent "None" (`KismetMathLibrary.Lerp` (`self.Min Mass`) (`self.Max Mass`) (`KismetMathLibrary.NormalizeToRange` _default_scale (`self.Min Scale`) (`self.Max Mass`))) true)
        (else
          (`PrimitiveComponent.SetMassScale` _staticmeshcomponent "None" _default_scale)))
      (`PrimitiveComponent.SetPhysicsLinearVelocity` _staticmeshcomponent (0.0 0.0 0.0) false "None")
      (`PrimitiveComponent.SetPhysicsAngularVelocityInDegrees` _staticmeshcomponent (0.0 0.0 0.0) false "None")
      (`self.K2_SetActorLocationAndRotation` (`self.K2_GetActorLocation` _respawnpoint) (`self.K2_GetActorRotation` _respawnpoint))
      (if (`self.Being Held`)
        (bind _asfirst_person_character (cast `/Game/MainGame/Blueprints/FirstPersonCharacter` (`GameplayStatics.GetPlayerPawn` 0)))
        (`/Game/MainGame/Blueprints/FirstPersonCharacter.Force Drop Component` _asfirst_person_character)))
    (:`Is Not Valid`
      (`self.K2_DestroyActor`))))

(event `Grow`
  (bind _max_scale (`self.Max Scale`))
  (bind _staticmeshcomponent (`self.StaticMeshComponent`))
  (bind _min_mass (`self.Min Mass`))
  (bind _overlappingactors (`PrimitiveComponent.GetOverlappingActors` (`self.Box1`) "/Script/Engine.StaticMeshActor"))
  (bind _returnvalue (`KismetMathLibrary.NormalizeToRange` (.x (`self.GetActorScale3D`)) (`self.Min Scale`) _max_scale))
  (bind _returnvalue_2 (+ (`self.GetActorScale3D`) (`KismetMathLibrary.Conv_DoubleToVector` (`self.Growth Rate`))))
  ;[1 1 1] Custom Events
  ;;[0.08239 1 0.2273] Grow
  (set `self.Overlapped Blocks` 0)
  (if (`self.Scaleable`)
    (for _array_element _overlappingactors
      (cast `/Game/MainGame/Blueprints/InteractiveObjects/Pickup_Block` _array_element)
      (`/Engine/EditorBlueprintResources/StandardMacros.IncrementInt` (`self.Overlapped Blocks`)))
    (if (not (> (- (`KismetArrayLibrary.Array_Length` _overlappingactors) (`self.Overlapped Blocks`)) 1))
      (if (or (>= (.x _returnvalue_2) _max_scale) (>= (.y _returnvalue_2) _max_scale) (>= (.z _returnvalue_2) _max_scale))
        (`self.SetActorScale3D` (`KismetMathLibrary.Conv_DoubleToVector` _max_scale))
        (else
          (`self.SetActorScale3D` _returnvalue_2)))
      (if (and (> _min_mass 0.0) (> (`self.Max Mass`) _min_mass))
        (`PrimitiveComponent.SetMassOverrideInKg` _staticmeshcomponent "None" (`KismetMathLibrary.Lerp` (`self.Min Mass`) (`self.Max Mass`) _returnvalue) true)
        (else
          (`PrimitiveComponent.SetMassScale` _staticmeshcomponent "None" (`KismetMathLibrary.Lerp` (`self.Min Scale`) (`self.Max Scale`) _returnvalue)))))))

(event `Shrink`
  (bind _min_scale (`self.Min Scale`))
  (bind _staticmeshcomponent (`self.StaticMeshComponent`))
  (bind _min_mass (`self.Min Mass`))
  (bind _returnvalue (`KismetMathLibrary.NormalizeToRange` (.x (`self.GetActorScale3D`)) (`self.Min Scale`) (`self.Max Scale`)))
  (bind _returnvalue_2 (+ (`self.GetActorScale3D`) (`KismetMathLibrary.Conv_DoubleToVector` (`self.Shrink Rate`))))
  ;[1 1 1] Custom Events
  ;;[0.05004 0.7393 0.9608] Shrink
  (if (`self.Scaleable`)
    (if (or (<= (.x _returnvalue_2) _min_scale) (<= (.y _returnvalue_2) _min_scale) (<= (.z _returnvalue_2) _min_scale))
      (`self.SetActorScale3D` (`KismetMathLibrary.Conv_DoubleToVector` _min_scale))
      (else
        (`self.SetActorScale3D` _returnvalue_2)))
    (if (and (> _min_mass 0.0) (> (`self.Max Mass`) _min_mass))
      (`PrimitiveComponent.SetMassOverrideInKg` _staticmeshcomponent "None" (`KismetMathLibrary.Lerp` (`self.Min Mass`) (`self.Max Mass`) _returnvalue) true)
      (else
        (`PrimitiveComponent.SetMassScale` _staticmeshcomponent "None" (`KismetMathLibrary.Lerp` (`self.Min Scale`) (`self.Max Scale`) _returnvalue))))))

(fn `?Player Collision`
  (returns (`Player Collision` :type Boolean))
  (return (`self.Player Collision`)))

(fn `?Scaleable`
  (returns (Scaleable :type Boolean))
  (return (`self.Scaleable`)))

(fn `Constrain Velocity`
  (bind _max_velocity (`self.Max Velocity`))
  (bind _returnvalue (`PrimitiveComponent.GetPhysicsLinearVelocity` (`self.StaticMeshComponent`) "None"))
  (bind _returnvalue_2 (`KismetMathLibrary.VSize` _returnvalue))
  (if (< _max_velocity _returnvalue_2)
    (`PrimitiveComponent.SetPhysicsLinearVelocity` (`self.StaticMeshComponent`) (* _returnvalue (/ _max_velocity _returnvalue_2)) false "None")))

(fn `SetBeingHeld`
  (params (NewHeld :type Boolean))
  (set `self.Being Held` NewHeld))

(fn `SetCanPickup`
  (params (`New Pickup` :type Boolean))
  (set `self.Force Non Pickup` `New Pickup`))

(fn `SetSpawn`
  (params (NewSpawnpoint :type "/Game/MainGame/Blueprints/Points/Pickup_BlockSpawnpoint Object Reference"))
  (`/Engine/EditorBlueprintResources/StandardMacros.IsValid` NewSpawnpoint
    (:`Is Valid`
      (set `self.RespawnPoint` NewSpawnpoint))))

(fn `UserConstructionScript`)