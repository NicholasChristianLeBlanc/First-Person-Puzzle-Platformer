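; Moving crusher platform that travels back and forth along an array of target actors and kills any FirstPersonCharacter that overlaps it.
; Tick drives a timeline with play rate based on remaining distance and MovementSpeed, lerping from the current location toward the target with sweep.
; When the timeline finishes, SetNextTarget steps through the array, reversing direction at either end.
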(event `self.ReceiveBeginPlay`
  (bind _targets (`self.Targets`))
  (if (> (`KismetArrayLibrary.Array_Length` _targets) 0)
    (set `self.Next Target` (`|GetArrayItem` _targets))))

(event `self.ReceiveTick`
  (params (DeltaSeconds :type "Float (single-precision)"))
  (bind _next_target (`self.Next Target`))
  (`TimelineComponent.SetPlayRate` (`self.Smooth Movement Graph`) (/ 1.0 (/ (`KismetMathLibrary.Abs` (`self.GetDistanceTo` _next_target)) (`self.Movement Speed`))))
  (bind (_direction _alpha) (`Timeline|Smooth Movement Graph` :!label _label)
    (:`Update`
      (`self.K2_SetActorLocation` (`KismetMathLibrary.VLerp` (`self.K2_GetActorLocation`) (`SceneComponent.K2_GetComponentLocation` (`Actor.RootComponent` _next_target)) _alpha) true))
    (:`Finished`
      (`self.Set Next Target`)
      (goto _label :!via `SetNewTime`))))

(event `self.ReceiveActorBeginOverlap`
  (params (OtherActor :type "Actor Object Reference"))
  (bind _asfirst_person_character (cast `/Game/MainGame/Blueprints/FirstPersonCharacter` OtherActor))
  (`/Game/MainGame/Blueprints/FirstPersonCharacter.Kill` _asfirst_person_character))

(fn `Set Next Target`
  (bind _targets (`self.Targets`))
  (for (_array_element _array_index) _targets
    (if (== _array_element (`self.Next Target`))
      (if (`self.Moving Forward`)
        (bind _returnvalue (+ _array_index 1))
        (if (not (> _returnvalue (- (`KismetArrayLibrary.Array_Length` _targets) 1)))
          _
          (else
            (bind _returnvalue_2 (- _array_index 1))
            (set `self.Next Target` (`|GetArrayItem` _targets _returnvalue_2) :!label _label)
            (set `self.Moving Forward` false)
            (break)))
        (elif (not (< _returnvalue_2 0))
          (goto _label)
          (else
            _)))
      (set `self.Next Target` (`|GetArrayItem` _targets _returnvalue))
      (set `self.Moving Forward` true)
      (break))))

(fn `UserConstructionScript`)