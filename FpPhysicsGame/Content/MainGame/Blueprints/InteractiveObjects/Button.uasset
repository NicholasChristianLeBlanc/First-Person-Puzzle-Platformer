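; Interactable button that switches linked puzzle objects such as doors, launch pads, force fields, spawners, shooters and moving platforms.
; A sphere overlap enables input for the first-person character, and each Interact press replays a timeline moving the button between its start and Arrow positions.
; When the timeline finishes, it calls ActivateAll, or alternates with DeactivateAll through a FlipFlop unless OnlyActivate is set.
; DeactivateAll leaves block spawners and freeze shooters untouched.
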(event `self.ReceiveBeginPlay`
  (set `self.Default Button Location` (`self.K2_GetActorLocation`))
  (set `self.Pressed Button Location` (`SceneComponent.K2_GetComponentLocation` (`self.Arrow`)))
  (`TimelineComponent.SetPlayRate` (`self.Timeline_0`) 4.0))

(event `self.Sphere.OnComponentBeginOverlap`
  (params (OverlappedComponent :type "PrimitiveComponent Object Reference") (OtherActor :type "Actor Object Reference") (OtherComp :type "PrimitiveComponent Object Reference") (OtherBodyIndex :type Integer) (bFromSweep :type Boolean) (SweepResult :type "HitResult Structure (by ref)"))
  (cast `/Game/MainGame/Blueprints/FirstPersonCharacter` OtherActor)
  (`self.EnableInput` (`GameplayStatics.GetPlayerController` 0)))

(event `self.Sphere.OnComponentEndOverlap`
  (params (OverlappedComponent :type "PrimitiveComponent Object Reference") (OtherActor :type "Actor Object Reference") (OtherComp :type "PrimitiveComponent Object Reference") (OtherBodyIndex :type Integer))
  (cast `/Game/MainGame/Blueprints/FirstPersonCharacter` OtherActor)
  (`self.DisableInput` (`GameplayStatics.GetPlayerController` 0)))

(event `InputAction|Interact`
  (params (Key :type "Key Structure"))
  (:`Pressed`
    (bind _isa (`/Engine/EditorBlueprintResources/StandardMacros.FlipFlop`)
      (:`A`
        (bind (_direction _alpha) (`Timeline|Timeline_0` :!via `PlayFromStart` :!label _label)
          (:`Update`
            (`self.K2_SetActorLocation` (`KismetMathLibrary.VLerp` (`self.Default Button Location`) (`self.Pressed Button Location`) _alpha)))
          (:`Finished`
            (if (`self.Only Activate`)
              (`self.Activate All` :!label _label_2)
              (elif _isa
                (goto _label_2)
                (else
                  (`self.Deactivate All`)))))))
      (:`B`
        (goto _label :!via `PlayFromStart`)))))

(fn `Activate All`
  (for _array_element (`self.Linked Doors`)
    (`/Engine/EditorBlueprintResources/StandardMacros.IsValid` _array_element
      (:`Is Valid`
        (`/Game/MainGame/Blueprints/InteractiveObjects/Door.Set Active` _array_element true))))
  (for _array_element_2 (`self.Linked Launch Pads`)
    (`/Engine/EditorBlueprintResources/StandardMacros.IsValid` _array_element_2
      (:`Is Valid`
        (`/Game/MainGame/Blueprints/InteractiveObjects/LaunchPads.Set Active` _array_element_2 true))))
  (for _array_element_3 (`self.Linked Force Fields`)
    (`/Engine/EditorBlueprintResources/StandardMacros.IsValid` _array_element_3
      (:`Is Valid`
        (`/Game/MainGame/Blueprints/InteractiveObjects/ForceField.Set Active` _array_element_3 true))))
  (for _array_element_4 (`self.Linked Block Spawners`)
    (`/Engine/EditorBlueprintResources/StandardMacros.IsValid` _array_element_4
      (:`Is Valid`
        (`/Game/MainGame/Blueprints/Points/Pickup_BlockSpawnpoint.Activate` _array_element_4))))
  (for _array_element_5 (`self.Linked Freeze Shooters`)
    (`/Engine/EditorBlueprintResources/StandardMacros.IsValid` _array_element_5
      (:`Is Valid`
        (`/Game/MainGame/Blueprints/InteractiveObjects/FreezeShooter.Activate` _array_element_5))))
  (for _array_element_6 (`self.Linked Movement Glass`)
    (`/Engine/EditorBlueprintResources/StandardMacros.IsValid` _array_element_6
      (:`Is Valid`
        (`/Game/MainGame/Blueprints/InteractiveObjects/MovementGlass.Set Active` _array_element_6 true))))
  (for _array_element_7 (`self.Linked Movement Platforms`)
    (`/Engine/EditorBlueprintResources/StandardMacros.IsValid` _array_element_7
      (:`Is Valid`
        (`/Game/MainGame/Blueprints/InteractiveObjects/MovementPlatforms.Set Active` _array_element_7 true)))))

(fn `Deactivate All`
  (for _array_element (`self.Linked Doors`)
    (`/Engine/EditorBlueprintResources/StandardMacros.IsValid` _array_element
      (:`Is Valid`
        (`/Game/MainGame/Blueprints/InteractiveObjects/Door.Set Active` _array_element false))))
  (for _array_element_2 (`self.Linked Launch Pads`)
    (`/Engine/EditorBlueprintResources/StandardMacros.IsValid` _array_element_2
      (:`Is Valid`
        (`/Game/MainGame/Blueprints/InteractiveObjects/LaunchPads.Set Active` _array_element_2 false))))
  (for _array_element_3 (`self.Linked Force Fields`)
    (`/Engine/EditorBlueprintResources/StandardMacros.IsValid` _array_element_3
      (:`Is Valid`
        (`/Game/MainGame/Blueprints/InteractiveObjects/ForceField.Set Active` _array_element_3 false))))
  (for _array_element_4 (`self.Linked Movement Glass`)
    (`/Engine/EditorBlueprintResources/StandardMacros.IsValid` _array_element_4
      (:`Is Valid`
        (`/Game/MainGame/Blueprints/InteractiveObjects/MovementGlass.Set Active` _array_element_4 false))))
  (for _array_element_5 (`self.Linked Movement Platforms`)
    (`/Engine/EditorBlueprintResources/StandardMacros.IsValid` _array_element_5
      (:`Is Valid`
        (`/Game/MainGame/Blueprints/InteractiveObjects/MovementPlatforms.Set Active` _array_element_5 false)))))

(fn `UserConstructionScript`)