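; Falling platform actor that drops when the player or a sufficiently large object overlaps it.
; On overlap, it accepts either an exact FirstPersonCharacter class match or any actor scaled above a threshold on all three axes.
; It then waits an optional FallDelay and enables physics simulation on its Cube component, with no reset logic.
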(event `self.ReceiveActorBeginOverlap`
  (params (OtherActor :type "Actor Object Reference"))
  (bind (_returnvalue_x _returnvalue_y _returnvalue_z) (`KismetMathLibrary.BreakVector` (`self.GetActorScale3D` OtherActor)))
  (bind _fall_delay (`self.Fall Delay`))
  (if (== (`GameplayStatics.GetObjectClass` OtherActor) "/Game/MainGame/Blueprints/FirstPersonCharacter.FirstPersonCharacter_C")
    (if (not (not (> _fall_delay 0.0))) :!label _label
      (`KismetSystemLibrary.Delay` _fall_delay))
    (`PrimitiveComponent.SetSimulatePhysics` (`self.Cube`) true)
    (elif (and (> _returnvalue_x 1.5) (> _returnvalue_y 1.5) (> _returnvalue_z 1.5))
      (goto _label))))

(fn `UserConstructionScript`)