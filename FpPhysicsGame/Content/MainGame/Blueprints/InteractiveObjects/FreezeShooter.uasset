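; FreezeShooter is an interactive object that fires a burst of FreezeProjectile actors when activated.
; While active, Tick passes through a short Delay to pace shots, counting each spawn against NumberOfProjectiles.
; Projectiles spawn at the Arrow component, with random rotation within ProjectileSpread on every axis.
; After the burst, it waits ActiveDelay, then deactivates and resets the counter for the next activation.
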(event `Activate`
  (set `self.Active` true))

(event `self.ReceiveTick`
  (params (DeltaSeconds :type "Float (single-precision)"))
  (bind _loop_counter (`self.Loop Counter`))
  (if (`self.Active`)
    (`KismetSystemLibrary.Delay` 0.05)
    (if (>= (`self.Number of Projectiles`) _loop_counter)
      (set `self.Loop Counter` (+ _loop_counter 1))
      (`self.Spawn Projectiles`)
      (else
        (`KismetSystemLibrary.Delay` (`self.Active Delay`))
        (set `self.Active` false)
        (set `self.Loop Counter` 0)))))

(event `Spawn Projectiles`
  (bind _projectile_spread (`self.Projectile Spread`))
  (bind _arrow (`self.Arrow`))
  (bind _returnvalue (* -1 _projectile_spread))
  (`|SpawnActorFromClass` "/Game/MainGame/Blueprints/Projectiles/FreezeProjectile.FreezeProjectile_C" (`KismetMathLibrary.MakeTransform` (`SceneComponent.K2_GetComponentLocation` _arrow) (`KismetMathLibrary.ComposeRotators` (`SceneComponent.K2_GetComponentRotation` _arrow) (`KismetMathLibrary.MakeRotator` (`KismetMathLibrary.RandomFloatInRange` _returnvalue _projectile_spread) (`KismetMathLibrary.RandomFloatInRange` _returnvalue _projectile_spread) (`KismetMathLibrary.RandomFloatInRange` _returnvalue _projectile_spread)))) "AdjustIfPossibleButAlwaysSpawn" "OverrideRootScale" null null))

(fn `UserConstructionScript`)