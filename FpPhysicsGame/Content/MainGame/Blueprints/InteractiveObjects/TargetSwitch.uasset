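; Puzzle switch triggered by Pickup_Block contact or, optionally, by projectiles, which it destroys on impact.
; Triggering activates linked doors, launch pads, force fields, glass, platforms and spawners, reveals linked actors and reassigns block spawn points.
; Unless StayActive is set, retriggering deactivates only the movers, doors, pads and fields, optionally after an ActiveTime delay.
; With LockCollidedActor, Tick makes overlapping blocks heavy and unpickable, rescaling mass once they leave.
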(event `self.ReceiveHit`
  (params (MyComp :type "PrimitiveComponent Object Reference") (Other :type "Actor Object Reference") (OtherComp :type "PrimitiveComponent Object Reference") (bSelfMoved :type Boolean) (HitLocation :type "Vector Structure") (HitNormal :type "Vector Structure") (NormalImpulse :type "Vector Structure") (Hit :type "HitResult Structure (by ref)"))
  (bind _returnvalue (`GameplayStatics.GetObjectClass` Other))
  ;[1 1 1] Hit Event
  (if (== _returnvalue "/Game/MainGame/Blueprints/InteractiveObjects/Pickup_Block.Pickup_Block_C")
    (set `self.Overlapped Actor` Other)
    (`self.Was Triggered`)
    (goto _label :!via `Reset`)
    (elif (== _returnvalue "/Game/MainGame/Blueprints/Projectiles/CollisionProjectile.CollisionProjectile_C")
      (`self.K2_DestroyActor` Other)
      (if (`self.Projectile Triggers`)
        (`self.Was Triggered`)))))

(event `self.ReceiveActorBeginOverlap`
  (params (OtherActor :type "Actor Object Reference"))
  (bind _returnvalue (`GameplayStatics.GetObjectClass` OtherActor))
  ;[1 1 1] Overlap Events
  (if (== _returnvalue "/Game/MainGame/Blueprints/InteractiveObjects/Pickup_Block.Pickup_Block_C")
    (set `self.Overlapped Actor` OtherActor)
    (`self.Was Triggered`)
    (goto _label :!via `Reset`)
    (elif (== _returnvalue "/Game/MainGame/Blueprints/Projectiles/CollisionProjectile.CollisionProjectile_C")
      (`self.K2_DestroyActor` OtherActor)
      (if (`self.Projectile Triggers`)
        (`self.Was Triggered`)))))

(event `self.ReceiveActorEndOverlap`
  (params (OtherActor :type "Actor Object Reference"))
  ;[1 1 1] Overlap Events
  (if (== (`GameplayStatics.GetObjectClass` OtherActor) "/Game/MainGame/Blueprints/InteractiveObjects/Pickup_Block.Pickup_Block_C")
    (`self.Was Triggered`)))

(event `self.ReceiveTick`
  (params (DeltaSeconds :type "Float (single-precision)"))
  (bind _returnvalue (`PrimitiveComponent.IsOverlappingActor` (`self.Box1`) (`self.Overlapped Actor`)))
  ;[1 1 1] Tick
  (if (`self.Lock Collided Actor`)
    (if (not _returnvalue)
      (`/Engine/EditorBlueprintResources/StandardMacros.DoOnce` false :!label _label
        (:`Completed`
          (`self.Unlock Collided Object`)))
      (else
        (`self.Lock Collided Object`)
        ;[1 0.1094 0.1094] Was Triggered
        (set `self.Was Hit` true :!label _label_2)
        (`/Engine/EditorBlueprintResources/StandardMacros.DoOnce` false :!label _label_3
          (:`Completed`
            (`self.Activate All`)
            (`self.Activate Spawners`)))))
    (elif (and _returnvalue (> (`KismetMathLibrary.Abs` (`self.Active Time`)) 0.0))
      (goto _label_2))))

(event `Was Triggered`
  (bind _returnvalue (`KismetMathLibrary.Abs` (`self.Active Time`)))
  ;[1 0.1094 0.1094] Was Triggered
  (if (not (`self.Was Hit`))
    (goto _label_2)
    (elif (not (`self.Stay Active`))
      (if (not (not (and (not (`PrimitiveComponent.IsOverlappingActor` (`self.Box1`) (`self.Overlapped Actor`))) (> _returnvalue 0.0))))
        (`KismetSystemLibrary.Delay` _returnvalue))
      (set `self.Was Hit` false)
      (`self.Deactivate All`)
      (goto _label_3 :!via `Reset`))))

(fn `Activate All`
  (for _array_element (`self.BlockChangeSpawn`)
    (bind (_pickup_block _spawnpoint) (break `/Game/MainGame/Assets/Structures/InteractiveObjects/Block_Spawnpoint_Reference` _array_element))
    (if (and (`KismetSystemLibrary.IsValid` _pickup_block) (`KismetSystemLibrary.IsValid` _spawnpoint))
      (`/Game/MainGame/Blueprints/InteractiveObjects/Pickup_Block.SetSpawn` _pickup_block _spawnpoint)))
  (for _array_element_2 (`self.Linked Doors`)
    (`/Engine/EditorBlueprintResources/StandardMacros.IsValid` _array_element_2
      (:`Is Valid`
        (`/Game/MainGame/Blueprints/InteractiveObjects/Door.Set Active` _array_element_2 true))))
  (for _array_element_3 (`self.Linked LaunchPads`)
    (`/Engine/EditorBlueprintResources/StandardMacros.IsValid` _array_element_3
      (:`Is Valid`
        (`/Game/MainGame/Blueprints/InteractiveObjects/LaunchPads.Set Active` _array_element_3 true))))
  (for _array_element_4 (`self.Linked ForceFields`)
    (`/Engine/EditorBlueprintResources/StandardMacros.IsValid` _array_element_4
      (:`Is Valid`
        (`/Game/MainGame/Blueprints/InteractiveObjects/ForceField.Trigger Change` _array_element_4))))
  (for _array_element_5 (`self.Linked MovementGlass`)
    (`/Engine/EditorBlueprintResources/StandardMacros.IsValid` _array_element_5
      (:`Is Valid`
        (`/Game/MainGame/Blueprints/InteractiveObjects/MovementGlass.Set Active` _array_element_5 true))))
  (for _array_element_6 (`self.Linked MovementPlatforms`)
    (`/Engine/EditorBlueprintResources/StandardMacros.IsValid` _array_element_6
      (:`Is Valid`
        (`/Game/MainGame/Blueprints/InteractiveObjects/MovementPlatforms.Set Active` _array_element_6 true))))
  (for _array_element_7 (`self.Linked Actor`)
    (`/Engine/EditorBlueprintResources/StandardMacros.IsValid` _array_element_7
      (:`Is Valid`
        (`self.SetActorHiddenInGame` _array_element_7 false)))))

(fn `Activate Spawners`
  (for _array_element (`self.Linked BlockSpawners`)
    (`/Engine/EditorBlueprintResources/StandardMacros.IsValid` _array_element
      (:`Is Valid`
        (`/Game/MainGame/Blueprints/Points/Pickup_BlockSpawnpoint.Activate` _array_element))))
  (for _array_element_2 (`self.Linked FreezeShooters`)
    (`/Engine/EditorBlueprintResources/StandardMacros.IsValid` _array_element_2
      (:`Is Valid`
        (`/Game/MainGame/Blueprints/InteractiveObjects/FreezeShooter.Activate` _array_element_2))))
  (for _array_element_3 (`self.Linked DeathWater`)
    (`/Engine/EditorBlueprintResources/StandardMacros.IsValid` _array_element_3
      (:`Is Valid`
        (`/Game/MainGame/Blueprints/InteractiveObjects/DeathWater.Activate` _array_element_3)))))

(fn `Deactivate All`
  (for _array_element (`self.Linked Doors`)
    (`/Engine/EditorBlueprintResources/StandardMacros.IsValid` _array_element
      (:`Is Valid`
        (`/Game/MainGame/Blueprints/InteractiveObjects/Door.Set Active` _array_element false))))
  (for _array_element_2 (`self.Linked LaunchPads`)
    (`/Engine/EditorBlueprintResources/StandardMacros.IsValid` _array_element_2
      (:`Is Valid`
        (`/Game/MainGame/Blueprints/InteractiveObjects/LaunchPads.Set Active` _array_element_2 false))))
  (for _array_element_3 (`self.Linked ForceFields`)
    (`/Engine/EditorBlueprintResources/StandardMacros.IsValid` _array_element_3
      (:`Is Valid`
        (`/Game/MainGame/Blueprints/InteractiveObjects/ForceField.Trigger Change` _array_element_3))))
  (for _array_element_4 (`self.Linked MovementGlass`)
    (`/Engine/EditorBlueprintResources/StandardMacros.IsValid` _array_element_4
      (:`Is Valid`
        (`/Game/MainGame/Blueprints/InteractiveObjects/MovementGlass.Set Active` _array_element_4 false))))
  (for _array_element_5 (`self.Linked MovementPlatforms`)
    (`/Engine/EditorBlueprintResources/StandardMacros.IsValid` _array_element_5
      (:`Is Valid`
        (`/Game/MainGame/Blueprints/InteractiveObjects/MovementPlatforms.Set Active` _array_element_5 false)))))

(fn `Get Active`
  (returns (`Is Active` :type Boolean))
  (return (`self.Was Hit`)))

(fn `Lock Collided Object`
  (bind _overlapped_actor (`self.Overlapped Actor`))
  (`/Engine/EditorBlueprintResources/StandardMacros.IsValid` _overlapped_actor
    (:`Is Valid`
      (bind _aspickup_block (cast `/Game/MainGame/Blueprints/InteractiveObjects/Pickup_Block` _overlapped_actor))
      (if (`PrimitiveComponent.IsOverlappingActor` (`self.Box1`) _overlapped_actor)
        (`/Game/MainGame/Blueprints/InteractiveObjects/Pickup_Block.SetCanPickup` _aspickup_block false)
        (`PrimitiveComponent.SetMassScale` (`StaticMeshActor.StaticMeshComponent` _aspickup_block) "None" 100.0)))))

(fn `Unlock Collided Object`
  (bind _overlapped_actor (`self.Overlapped Actor`))
  (`/Engine/EditorBlueprintResources/StandardMacros.IsValid` _overlapped_actor
    (:`Is Valid`
      (bind _aspickup_block (cast `/Game/MainGame/Blueprints/InteractiveObjects/Pickup_Block` _overlapped_actor))
      (if (not (`PrimitiveComponent.IsOverlappingActor` (`self.Box1`) _overlapped_actor))
        (bind _staticmeshcomponent (`StaticMeshActor.StaticMeshComponent` _aspickup_block))
        (bind _returnvalue_x (`KismetMathLibrary.BreakVector` (`SceneComponent.K2_GetComponentScale` _staticmeshcomponent)))
        (`PrimitiveComponent.SetMassScale` _staticmeshcomponent "None" (* (/ (`PrimitiveComponent.GetMassScale` _staticmeshcomponent "None") 100.0) _returnvalue_x))))))

(fn `UserConstructionScript`)