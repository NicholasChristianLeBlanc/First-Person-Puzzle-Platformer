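; DeathWater is a lethal water volume that can rise and fall between flood and drain waypoints.
; Its box kills the player, respawns block pickups and destroys collision, grow and shrink projectiles on overlap.
; Activate ignores calls while animating, otherwise choosing Flood or Drain by current height; Flood first destroys overlapping FreezePlatforms.
; Timelines lerp from the current location, snapping near the target, with play rates optionally scaled by distance.
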(event `self.ReceiveBeginPlay`
  (bind _flood_rate (`self.Flood Rate`))
  (bind _flood_waypoint (`self.Flood Waypoint`))
  (bind _drain_waypoint (`self.Drain Waypoint`))
  (bind _drain_rate (`self.Drain Rate`))
  (bind _drain_timeline (`self.Drain Timeline`))
  (bind _flood_waypoint_2 (`self.Flood Waypoint`))
  (bind _drain_waypoint_2 (`self.Drain Waypoint`))
  (bind _flood_timeline (`self.Flood Timeline`))
  (`/Engine/EditorBlueprintResources/StandardMacros.IsValid` _flood_waypoint
    (:`Is Valid`
      (if (not (`self.Flood Rate By Distance`))
        (`TimelineComponent.SetPlayRate` _flood_timeline (`self.Flood Rate`))
        (elif (not (`KismetSystemLibrary.IsValid` _drain_waypoint))
          (`TimelineComponent.SetPlayRate` _flood_timeline (/ 1.0 (/ (`KismetMathLibrary.Abs` (`self.GetDistanceTo` _flood_waypoint)) _flood_rate)))
          (else
            (`TimelineComponent.SetPlayRate` _flood_timeline (/ 1.0 (/ (`KismetMathLibrary.Abs` (`self.GetDistanceTo` _flood_waypoint _drain_waypoint)) _flood_rate))))))
      (`/Engine/EditorBlueprintResources/StandardMacros.IsValid` _drain_waypoint_2
        (:`Is Valid`
          (if (not (`self.Drain Rate By Distance`))
            (`TimelineComponent.SetPlayRate` _drain_timeline (`self.Drain Rate`))
            (elif (not (`KismetSystemLibrary.IsValid` _flood_waypoint_2))
              (`TimelineComponent.SetPlayRate` _drain_timeline (/ 1.0 (/ (`KismetMathLibrary.Abs` (`self.GetDistanceTo` _drain_waypoint_2)) _drain_rate)))
              (else
                (`TimelineComponent.SetPlayRate` _drain_timeline (/ 1.0 (/ (`KismetMathLibrary.Abs` (`self.GetDistanceTo` _drain_waypoint_2 _flood_waypoint_2)) _drain_rate)))))))))))

(event `self.Box.OnComponentBeginOverlap`
  (params (OverlappedComponent :type "PrimitiveComponent Object Reference") (OtherActor :type "Actor Object Reference") (OtherComp :type "PrimitiveComponent Object Reference") (OtherBodyIndex :type Integer) (bFromSweep :type Boolean) (SweepResult :type "HitResult Structure (by ref)"))
  (bind _returnvalue (`GameplayStatics.GetObjectClass` OtherActor))
  (bind _asfirst_person_character (cast `/Game/MainGame/Blueprints/FirstPersonCharacter` OtherActor)
    (:`then`
      (`/Game/MainGame/Blueprints/FirstPersonCharacter.Kill` _asfirst_person_character))
    (:`CastFailed`
      (bind _aspickup_block (cast `/Game/MainGame/Blueprints/InteractiveObjects/Pickup_Block` OtherActor)
        (:`then`
          (if (== OtherComp (`/Game/MainGame/Blueprints/InteractiveObjects/Pickup_Block.Box` _aspickup_block))
            (`/Game/MainGame/Blueprints/InteractiveObjects/Pickup_Block.Respawn` _aspickup_block)))
        (:`CastFailed`
          (if (or (== _returnvalue "/Game/MainGame/Blueprints/Projectiles/CollisionProjectile.CollisionProjectile_C") (== _returnvalue "/Game/MainGame/Blueprints/Projectiles/GrowProjectile.GrowProjectile_C") (== _returnvalue "/Game/MainGame/Blueprints/Projectiles/ShrinkProjectile.ShrinkProjectile_C"))
            (`self.K2_DestroyActor` OtherActor)))))))

(event `Drain`
  (bind _returnvalue (`self.K2_GetActorLocation`))
  (bind _drain_waypoint (`self.Drain Waypoint`))
  (bind _returnvalue_2 (`self.K2_GetActorLocation` _drain_waypoint))
  (set `self.Animating` true)
  (bind (_direction _alpha) (`Timeline|Drain Timeline` :!via `PlayFromStart` :!label _label)
    (:`Update`
      (`/Engine/EditorBlueprintResources/StandardMacros.IsValid` _drain_waypoint
        (:`Is Valid`
          (if (not (<= (.z _returnvalue) (+ (.z _returnvalue_2) 0.7)))
            (`self.K2_SetActorLocation` (`KismetMathLibrary.VLerp` _returnvalue _returnvalue_2 _alpha) true)
            (else
              (`self.K2_SetActorLocation` _returnvalue_2 true)
              (set `self.Animating` false)
              (goto _label :!via `Stop`))))))))

(event `Flood`
  (bind _returnvalue (`self.K2_GetActorLocation`))
  (bind _flood_waypoint (`self.Flood Waypoint`))
  (bind _returnvalue_2 (`self.K2_GetActorLocation` _flood_waypoint))
  (bind _outactors (`GameplayStatics.GetAllActorsOfClass` "/Game/MainGame/Blueprints/InteractiveObjects/FreezePlatform.FreezePlatform_C"))
  (for _array_element _outactors
    (if (`PrimitiveComponent.IsOverlappingActor` (`self.Box`) _array_element)
      (`self.K2_DestroyActor` _array_element)))
  (set `self.Animating` true)
  (bind (_direction _alpha) (`Timeline|Flood Timeline` :!via `PlayFromStart` :!label _label_2)
    (:`Update`
      (`/Engine/EditorBlueprintResources/StandardMacros.IsValid` _flood_waypoint
        (:`Is Valid`
          (if (not (>= (.z _returnvalue) (- (.z _returnvalue_2) 0.7)))
            (`self.K2_SetActorLocation` (`KismetMathLibrary.VLerp` _returnvalue _returnvalue_2 _alpha) true)
            (else
              (`self.K2_SetActorLocation` _returnvalue_2 true)
              (set `self.Animating` false)
              (goto _label_2 :!via `Stop`))))))))

(fn `Activate`
  (bind (_returnvalue_x _returnvalue_y _returnvalue_z) (`KismetMathLibrary.BreakVector` (`self.K2_GetActorLocation`)))
  (bind (_returnvalue_x_2 _returnvalue_y_2 _returnvalue_z_2) (`KismetMathLibrary.BreakVector` (`self.K2_GetActorLocation`)))
  (bind _flood_waypoint (`self.Flood Waypoint`))
  (bind _drain_waypoint (`self.Drain Waypoint`))
  (bind (_returnvalue_x_3 _returnvalue_y_3 _returnvalue_z_3) (`KismetMathLibrary.BreakVector` (`self.K2_GetActorLocation` _drain_waypoint)))
  (bind (_returnvalue_x_4 _returnvalue_y_4 _returnvalue_z_4) (`KismetMathLibrary.BreakVector` (`self.K2_GetActorLocation` _flood_waypoint)))
  (if (not (`self.Animating`))
    (`/Engine/EditorBlueprintResources/StandardMacros.IsValid` _flood_waypoint
      (:`Is Valid`
        (if (not (>= _returnvalue_z_2 _returnvalue_z_4))
          (`self.Flood`)
          (else
            (`/Engine/EditorBlueprintResources/StandardMacros.IsValid` _drain_waypoint :!label _label
              (:`Is Valid`
                (if (not (<= _returnvalue_z _returnvalue_z_3))
                  (`self.Drain`)))))))
      (:`Is Not Valid`
        (goto _label)))))

(fn `UserConstructionScript`)