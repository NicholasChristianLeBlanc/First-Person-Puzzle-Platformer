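; A gun pickup table that arms the first-person character when they walk into it.
; On sphere overlap it hides the table's gun mesh, calls deactivate on the collider and makes the character's gun visible.
; A separate IsObservable helper, not called in this graph, line-traces on Visibility from a skeletal mesh to the player controller's location and returns true when nothing blocks it.
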(event `self.Sphere Collider.OnComponentBeginOverlap`
  (params (OverlappedComponent :type "PrimitiveComponent Object Reference") (OtherActor :type "Actor Object Reference") (OtherComp :type "PrimitiveComponent Object Reference") (OtherBodyIndex :type Integer) (bFromSweep :type Boolean) (SweepResult :type "HitResult Structure (by ref)"))
  (bind _asfirst_person_character (cast `/Game/MainGame/Blueprints/FirstPersonCharacter` OtherActor))
  (`SceneComponent.SetHiddenInGame` (`self.Gun Mesh`) true false)
  (`ActorComponent.SetActive` (`self.Sphere Collider`) false false)
  (`/Game/MainGame/Blueprints/FirstPersonCharacter.Set Gun Visible` _asfirst_person_character true))

(fn `Is Observable`
  (params (`Skeletal Mesh` :type "SkeletalMeshComponent Object Reference"))
  (returns (`Is Observable` :type Boolean))
  (bind (_outhit _returnvalue) (`KismetSystemLibrary.LineTraceSingle` :`Start` (`SceneComponent.K2_GetComponentLocation` `Skeletal Mesh`) :`End` (`self.K2_GetActorLocation` (`GameplayStatics.GetPlayerController` 0)) :`TraceChannel` "TraceTypeQuery1" :`bIgnoreSelf` false))
  (return (not _returnvalue)))

(fn `UserConstructionScript`)