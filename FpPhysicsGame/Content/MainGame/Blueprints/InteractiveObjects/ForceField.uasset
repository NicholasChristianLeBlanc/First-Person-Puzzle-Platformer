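; ForceField is an overlap barrier that, while active, either kills the player or filters objects, depending on KillPlayer.
; In kill mode it only kills the FirstPersonCharacter; otherwise it destroys grow, shrink and freeze projectiles and respawns Pickup_Blocks.
; TriggerChange flips either the active state or kill mode according to Mode.
; Active controls visibility and gates the overlap response, while UpdateMaterial swaps the cube's material to match kill mode.
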(event `self.ReceiveBeginPlay`
  (`self.Update Material`)
  (`self.Set Active` (`self.Active`)))

(event `self.ReceiveActorBeginOverlap`
  (params (OtherActor :type "Actor Object Reference"))
  (bind _returnvalue (`GameplayStatics.GetObjectClass` OtherActor))
  (if (`self.Active`)
    (if (`self.Kill Player`)
      (bind _asfirst_person_character (cast `/Game/MainGame/Blueprints/FirstPersonCharacter` OtherActor))
      (`/Game/MainGame/Blueprints/FirstPersonCharacter.Kill` _asfirst_person_character)
      (elif (not (or (== _returnvalue "/Game/MainGame/Blueprints/Projectiles/GrowProjectile.GrowProjectile_C") (== _returnvalue "/Game/MainGame/Blueprints/Projectiles/ShrinkProjectile.ShrinkProjectile_C") (== _returnvalue "/Game/MainGame/Blueprints/Projectiles/FreezeProjectile.FreezeProjectile_C")))
        (bind _aspickup_block (cast `/Game/MainGame/Blueprints/InteractiveObjects/Pickup_Block` OtherActor))
        (`/Game/MainGame/Blueprints/InteractiveObjects/Pickup_Block.Respawn` _aspickup_block)
        (else
          (`self.K2_DestroyActor` OtherActor))))))

(fn `Set Active`
  (params (NewActive :type Boolean))
  (bind _output_get (set `self.Active` NewActive))
  (`self.SetActorHiddenInGame` (not _output_get)))

(fn `Set Kill Player`
  (params (`New Kill Player` :type Boolean))
  (set `self.Kill Player` `New Kill Player`))

(fn `Trigger Active`
  (bind _output_get (set `self.Active` (not (`self.Active`))))
  (`self.SetActorHiddenInGame` (not _output_get)))

(fn `Trigger Change`
  (switch `/Game/MainGame/Assets/Enums/Interactable_Objects/ForceFieldModes` (`self.Mode`)
    (:`NewEnumerator0`
      (`self.Trigger Active`))
    (:`NewEnumerator3`
      (`self.Trigger Kill Player`)
      (`self.Update Material`))))

(fn `Trigger Kill Player`
  (set `self.Kill Player` (not (`self.Kill Player`)))
  (`self.Update Material`))

(fn `Update Material`
  (bind _player_material (`self.Player Material`))
  (bind _default_material (`self.Default Material`))
  (bind _cube (`self.Cube`))
  (bind _returnvalue (`MeshComponent.GetMaterials` (`self.Cube`)))
  (if (`self.Kill Player`)
    (`/Engine/EditorBlueprintResources/StandardMacros.IsValid` _player_material
      (:`Is Valid`
        (if (not (`KismetArrayLibrary.Array_Contains` _returnvalue _player_material))
          (`PrimitiveComponent.SetMaterial` _cube 0 (`self.Player Material`)))))
    (else
      (`/Engine/EditorBlueprintResources/StandardMacros.IsValid` _default_material
        (:`Is Valid`
          (if (not (`KismetArrayLibrary.Array_Contains` _returnvalue _default_material))
            (`PrimitiveComponent.SetMaterial` _cube 0 (`self.Default Material`))))))))

(fn `UserConstructionScript`)