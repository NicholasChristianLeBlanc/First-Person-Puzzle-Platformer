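; A force field actor that kills the first-person character on overlap while it is effectively on.
; An InvertActive flag flips the meaning of Active, so the field can be on when Active is false.
; BeginPlay and SetActive show or hide the actor to match that state.
; Collision is never toggled; the overlap event checks both flags before calling Kill on the character.
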(event `self.ReceiveBeginPlay`
  (bind _active (`self.Active`))
  (if (not (`self.Invert Active`))
    (if _active
      (`self.SetActorHiddenInGame` false :!label _label)
      (else
        (`self.SetActorHiddenInGame` true :!label _label_2)))
    (elif (not _active)
      (goto _label)
      (else
        (goto _label_2)))))

(event `self.ReceiveActorBeginOverlap`
  (params (OtherActor :type "Actor Object Reference"))
  (bind _active (`self.Active`))
  (if (not (`self.Invert Active`))
    (if _active
      (bind _asfirst_person_character (cast `/Game/MainGame/Blueprints/FirstPersonCharacter` OtherActor :!label _label_3))
      (`/Game/MainGame/Blueprints/FirstPersonCharacter.Kill` _asfirst_person_character))
    (elif (not _active)
      (goto _label_3))))

(fn `Set Active`
  (params (`New Active` :type Boolean))
  (bind _output_get (set `self.Active` `New Active`))
  (if (`self.Invert Active`)
    (if _output_get
      (`self.SetActorHiddenInGame` true :!label _label)
      (else
        (`self.SetActorHiddenInGame` false :!label _label_2)))
    (elif _output_get
      (goto _label_2)
      (else
        (goto _label)))))

(fn `UserConstructionScript`)