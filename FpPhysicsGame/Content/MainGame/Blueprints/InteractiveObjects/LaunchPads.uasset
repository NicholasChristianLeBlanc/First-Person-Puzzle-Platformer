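; A launch pad actor that, while active, throws overlapping first-person characters or physics-simulating pickup blocks.
; Box overlap sends a calculated launch velocity to either the block's custom Launch or LaunchCharacter with full velocity override.
; With a valid Waypoint, Tick plays a timeline while active, lerping the pad from its start position to the waypoint, and reverses it when inactive.
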(event `self.ReceiveBeginPlay`
  (set `self.Default Position` (`self.K2_GetActorLocation`)))

(event `self.Box.OnComponentBeginOverlap`
  (params (OverlappedComponent :type "PrimitiveComponent Object Reference") (OtherActor :type "Actor Object Reference") (OtherComp :type "PrimitiveComponent Object Reference") (OtherBodyIndex :type Integer) (bFromSweep :type Boolean) (SweepResult :type "HitResult Structure (by ref)"))
  (bind _forward_velocity (`self.Forward Velocity`))
  (bind (_returnvalue_x _returnvalue_y) (`KismetMathLibrary.BreakVector` (`KismetMathLibrary.GetForwardVector` (`SceneComponent.K2_GetComponentRotation` (`self.Arrow`)))))
  (bind _returnvalue (* (`KismetMathLibrary.MakeVector` (* _forward_velocity _returnvalue_x) (* _forward_velocity _returnvalue_y) (`KismetMathLibrary.Abs` (`self.Upwards Velocity`))) 1000.0))
  (if (`self.Active`)
    (if (`SceneComponent.IsSimulatingPhysics` OtherComp "None")
      (bind _aspickup_block (cast `/Game/MainGame/Blueprints/InteractiveObjects/Pickup_Block` OtherActor))
      (`/Game/MainGame/Blueprints/InteractiveObjects/Pickup_Block.Launch` _aspickup_block _returnvalue)
      (else
        (bind _asfirst_person_character (cast `/Game/MainGame/Blueprints/FirstPersonCharacter` OtherActor))
        (`Character.LaunchCharacter` _asfirst_person_character _returnvalue true true)))))

(event `self.ReceiveTick`
  (params (DeltaSeconds :type "Float (single-precision)"))
  (`/Engine/EditorBlueprintResources/StandardMacros.IsValid` (`self.Waypoint`)
    (:`Is Valid`
      (if (`self.Active`)
        (bind (_direction _alpha) (`Timeline|Timeline_0` :!label _label)
          (:`Update`
            (`self.K2_SetActorLocation` (`KismetMathLibrary.VLerp` (`self.Default Position`) (`SceneComponent.K2_GetComponentLocation` (`Actor.RootComponent` (`self.Waypoint`))) _alpha))))
        (else
          (goto _label :!via `Reverse`))))))

(fn `Set Active`
  (params (`New Active` :type Boolean))
  (set `self.Active` `New Active`))

(fn `UserConstructionScript`)