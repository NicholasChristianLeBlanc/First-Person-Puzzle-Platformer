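; Interactive door that slides between its starting position and an OpenLocation marker based on the Active flag set through SetActive.
; Tick polls that flag to play or reverse a timeline that lerps the root with sweep, and CloseOnActive inverts the response.
; With DoorFailure set on a non-inverted door, activation instead plays a failure timeline with a scale-based vertical offset, timed spark bursts and looping sparks on finish.
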(event `self.ReceiveBeginPlay`
  (set `self.Default Position` (`self.K2_GetActorLocation`))
  (set `self.Open Position` (`SceneComponent.K2_GetComponentLocation` (`self.Open Location`))))

(event `self.ReceiveTick`
  (params (DeltaSeconds :type "Float (single-precision)"))
  (bind (_returnvalue_x _returnvalue_y _returnvalue_z) (`KismetMathLibrary.BreakVector` (`self.GetActorScale3D`)))
  (bind _active (`self.Active`))
  (bind _default_position (`self.Default Position`))
  (if (`self.Close On Active`)
    (if (not _active)
      (bind (_direction _alpha) (`Timeline|Active Timeline` :!label _label)
        (:`Update`
          (`SceneComponent.K2_SetWorldLocation` (`self.DefaultSceneRoot`) (`KismetMathLibrary.VLerp` (`self.Default Position`) (`self.Open Position`) _alpha) true false)))
      (else
        (goto _label :!via `Reverse`)))
    (elif _active
      (if (not (`self.Door Failure`))
        (goto _label)
        (else
          (bind (_direction_2 _alpha_2) (`Timeline|Failure Timeline`)
            (:`Update`
              (if (and (>= _alpha_2 0.65) (<= _alpha_2 1.0))
                (`ActorComponent.SetActive` (`self.FailureSpark`) true false)
                (`ActorComponent.SetActive` (`self.FailureSpark1`) true false)
                (`ActorComponent.SetActive` (`self.FailureSpark2`) true false)
                (`ActorComponent.SetActive` (`self.FailureSpark3`) true false)
                (else
                  (`ActorComponent.SetActive` (`self.FailureSpark1`) false true)
                  (`ActorComponent.SetActive` (`self.FailureSpark`) false true)
                  (`ActorComponent.SetActive` (`self.FailureSpark3`) false true)
                  (`ActorComponent.SetActive` (`self.FailureSpark2`) false true)))
              (`SceneComponent.K2_SetWorldLocation` (`self.DefaultSceneRoot`) (`KismetMathLibrary.VLerp` _default_position (`KismetMathLibrary.TransformLocation` (`KismetMathLibrary.MakeTransform` (`KismetMathLibrary.MakeVector` 0.0 0.0 (* _returnvalue_z 75.25))) _default_position) _alpha_2) true false))
            (:`Finished`
              (`ActorComponent.Activate` (`self.LoopingSparks`) false)
              (`ActorComponent.Activate` (`self.LoopingSparks1`) false)
              (`ActorComponent.Activate` (`self.LoopingSparks2`) false)
              (`ActorComponent.Activate` (`self.LoopingSparks3`) false)))))
      (else
        (goto _label :!via `Reverse`)))))

(fn `Set Active`
  (params (`New Active` :type Boolean))
  (set `self.Active` `New Active`))

(fn `UserConstructionScript`)